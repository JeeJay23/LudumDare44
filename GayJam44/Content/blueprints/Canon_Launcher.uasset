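; Launcher actor that repeatedly fires Canon actors from its Spawn component at a fixed interval.
; Tick counts down a timer seeded from Interval, then spawns a Canon regardless of collision, resets the timer and activates the PExplosion effect.
; Each new Canon receives the launcher's CanonDirection.
; Unconnected debug print and sphere impulse nodes remain in the graph but never run.
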(event EventBeginPlay
  (Variables|Default|Settimer (Variables|Default|GetInterval)))

(event Collision|EventActorBeginOverlap
  (params (OtherActor :type Actor%20Object%20Reference)))

(event EventTick
  (params (DeltaSeconds :type Float%20%28single-precision%29))
  (if (<= (Variables|Default|Gettimer) 0.0)
    (bind _returnvalue (Game|SpawnActorfromClass "/Game/blueprints/Canon.Canon_C" (Transformation|GetWorldTransform (Variables|Default|GetSpawn)) "AlwaysSpawn" 0 0))
    (Variables|Default|Settimer (Variables|Default|GetInterval))
    (Components|Activation|Activate (Variables|Default|GetP_Explosion) true)
    (Variables|/Game/blueprints/Canon.Canon_C|SetDirection _returnvalue (Variables|Default|GetCanon%20Direction))
    (else
      (Variables|Default|Settimer (- (Variables|Default|Gettimer) DeltaSeconds)))))

(fn ConstructionScript)