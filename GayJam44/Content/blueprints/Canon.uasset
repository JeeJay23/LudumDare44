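; Canon actor that travels in a straight line for a limited time, then becomes a physics-simulated object.
; While Timer is above zero, Tick moves the actor by Direction scaled by delta time, keeping rotation and scale, and counts Timer down.
; When Timer runs out, the Sphere component starts simulating physics and switches to a hewn stone brick material.
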(event EventBeginPlay)

(event Collision|EventActorBeginOverlap
  (params (OtherActor :type Actor%20Object%20Reference)))

(event EventTick
  (params (DeltaSeconds :type Float%20%28single-precision%29))
  (bind _returnvalue (Transformation|GetActorLocation))
  (bind _direction (Variables|Default|GetDirection))
  (if (not (<= (Variables|Default|GetTimer) 0.0))
    (Transformation|SetActorTransform (Math|Transform|MakeTransform (Math|Vector|MakeVector (+ (* DeltaSeconds (.x _direction)) (.x _returnvalue)) (+ (* DeltaSeconds (.y _direction)) (.y _returnvalue)) (+ (* DeltaSeconds (.z _direction)) (.z _returnvalue))) (Transformation|GetActorRotation) (Transformation|GetActorScale3D)))
    (Variables|Default|SetTimer (- (Variables|Default|GetTimer) DeltaSeconds))
    (if (<= (Variables|Default|GetTimer) 0.0)
      (Physics|SetSimulatePhysics (Variables|Default|GetSphere) true)
      (Rendering|Material|SetMaterial (Variables|Default|GetSphere) 0 "/Game/StarterContent/Materials/M_Brick_Hewn_Stone.M_Brick_Hewn_Stone"))))

(fn ConstructionScript)