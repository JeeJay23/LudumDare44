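; Swinging hammer hazard actor that loops through raise, drop and rest phases after an initial HammerDelay, mirrored by the Right flag.
; Tick integrates roll from Speed and advances a five-phase State machine whenever roll passes RotationLimit.
; The drop compounds acceleration through SadMultiplier, enabling HurtboxTrigger while disabling both hammer collisions.
; At the bottom it snaps the rotation, restores collision and creeps briefly before rising again.
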(event EventBeginPlay
  (Variables|Default|SetSpeed (Variables|Default|GetHammer%20Speed%20Raise))
  (Variables|Default|SetSadMultiplier 1.0)
  (if (Variables|Default|GetRight)
    (Variables|Default|SetRotation%20Limit 45.0)
    (else
      (Variables|Default|SetRotation%20Limit -45.0))))

(event Collision|EventActorBeginOverlap
  (params (OtherActor :type Actor%20Object%20Reference)))

(event EventTick
  (params (DeltaSeconds :type Float%20%28single-precision%29))
  (bind _right (Variables|Default|GetRight))
  (if (<= (Variables|Default|GetHammer%20Delay) 0.0)
    (if (Variables|Default|GetHammer%20Drop)
      (Variables|Default|SetSadMultiplier (+ (Variables|Default|GetSadMultiplier) (/ DeltaSeconds 4.0)))
      (Variables|Default|SetSpeed (* (+ (* (* (Variables|Default|GetHammer%20Speed%20Drop) DeltaSeconds) (Variables|Default|GetHammer%20Drop%20Acceleration)) (Variables|Default|GetSpeed)) (Variables|Default|GetSadMultiplier))))
    (Transformation|SetActorTransform (Math|Transform|MakeTransform (Transformation|GetActorLocation) (Math|Rotator|MakeRotator (+ (* DeltaSeconds (Variables|Default|GetSpeed)) (.Roll (Math|Rotator|BreakRotator (Transformation|GetActorRotation)))) 0.0 0.0) (Transformation|GetActorScale3D)))
    (if (== (Variables|Default|GetState) 0)
      (if (Variables|Default|GetRight)
        (if (>= (.Roll (Math|Rotator|BreakRotator (Transformation|GetActorRotation))) (Variables|Default|GetRotation%20Limit))
          (Variables|Default|SetState 1 :!label _label)
          (Variables|Default|SetSpeed (/ (Variables|Default|GetHammer%20Speed%20Raise) 2.0))
          (if (Variables|Default|GetRight)
            (Variables|Default|SetRotation%20Limit 9e+01)
            (else
              (Variables|Default|SetRotation%20Limit -9e+01))))
        (elif (<= (.Roll (Math|Rotator|BreakRotator (Transformation|GetActorRotation))) (Variables|Default|GetRotation%20Limit))
          (goto _label)))
      (elif (== (Variables|Default|GetState) 1)
        (if (Variables|Default|GetRight)
          (if (>= (.Roll (Math|Rotator|BreakRotator (Transformation|GetActorRotation))) (Variables|Default|GetRotation%20Limit))
            (Variables|Default|SetState 2 :!label _label_2)
            (Variables|Default|SetSpeed (/ (Variables|Default|GetHammer%20Speed%20Drop) 2.0))
            (Variables|Default|SetHammer%20Drop true)
            (Collision|SetCollisionEnabled (Variables|Default|GetHurtbox%20Trigger) "QueryAndPhysics")
            (Collision|SetCollisionEnabled (Variables|Default|GetHammer%20Collisionn) "NoCollision")
            (Collision|SetCollisionEnabled (Variables|Default|GetHammer%20Collisionn%202) "NoCollision")
            (if (Variables|Default|GetRight)
              (Variables|Default|SetRotation%20Limit -9e+01)
              (else
                (Variables|Default|SetRotation%20Limit 9e+01))))
          (elif (<= (.Roll (Math|Rotator|BreakRotator (Transformation|GetActorRotation))) (Variables|Default|GetRotation%20Limit))
            (goto _label_2)))
        (elif (== (Variables|Default|GetState) 2)
          (if (Variables|Default|GetRight)
            (if (<= (.Roll (Math|Rotator|BreakRotator (Transformation|GetActorRotation))) (Variables|Default|GetRotation%20Limit))
              (Variables|Default|SetState 3 :!label _label_3)
              (Variables|Default|SetSpeed (* (Variables|Default|GetHammer%20Speed%20Raise) 0.01))
              (Collision|SetCollisionEnabled (Variables|Default|GetHurtbox%20Trigger) "NoCollision")
              (Collision|SetCollisionEnabled (Variables|Default|GetHammer%20Collisionn) "QueryAndPhysics")
              (Collision|SetCollisionEnabled (Variables|Default|GetHammer%20Collisionn%202) "QueryAndPhysics")
              (Variables|Default|SetHammer%20Drop false)
              (if _right
                (Transformation|SetActorTransform (Math|Transform|MakeTransform (Transformation|GetActorLocation) "0.000000, 0,-90.000000" (Transformation|GetActorScale3D)))
                (else
                  (Transformation|SetActorTransform (Math|Transform|MakeTransform (Transformation|GetActorLocation) "0.000000, 0,90.000000" (Transformation|GetActorScale3D)))))
              (Variables|Default|SetSadMultiplier 1.0)
              (if _right
                (Variables|Default|SetRotation%20Limit -89.599998)
                (else
                  (Variables|Default|SetRotation%20Limit 89.599998))))
            (elif (>= (.Roll (Math|Rotator|BreakRotator (Transformation|GetActorRotation))) (Variables|Default|GetRotation%20Limit))
              (goto _label_3)))
          (elif (== (Variables|Default|GetState) 3)
            (if (Variables|Default|GetRight)
              (if (>= (.Roll (Math|Rotator|BreakRotator (Transformation|GetActorRotation))) (Variables|Default|GetRotation%20Limit))
                (Variables|Default|SetState 4 :!label _label_4)
                (Variables|Default|SetSpeed (* (Variables|Default|GetHammer%20Speed%20Raise) 0.6))
                (Variables|Default|SetSadMultiplier 1.0)
                (if (Variables|Default|GetRight)
                  (Variables|Default|SetRotation%20Limit -89.599998)
                  (else
                    (Variables|Default|SetRotation%20Limit 89.599998))))
              (elif (<= (.Roll (Math|Rotator|BreakRotator (Transformation|GetActorRotation))) (Variables|Default|GetRotation%20Limit))
                (goto _label_4)))
            (elif (Variables|Default|GetRight)
              (if (>= (.Roll (Math|Rotator|BreakRotator (Transformation|GetActorRotation))) (Variables|Default|GetRotation%20Limit))
                (Variables|Default|SetState 0 :!label _label_5)
                (Variables|Default|SetSpeed (Variables|Default|GetHammer%20Speed%20Raise))
                (if (Variables|Default|GetRight)
                  (Variables|Default|SetRotation%20Limit 45.0)
                  (else
                    (Variables|Default|SetRotation%20Limit -45.0))))
              (elif (<= (.Roll (Math|Rotator|BreakRotator (Transformation|GetActorRotation))) (Variables|Default|GetRotation%20Limit))
                (goto _label_5)))))))
    (else
      (Variables|Default|SetHammer%20Delay (- (Variables|Default|GetHammer%20Delay) DeltaSeconds)))))

(fn ConstructionScript)